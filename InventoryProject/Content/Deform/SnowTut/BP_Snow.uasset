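; BP_Snow is a deformable snow surface that records footprints in a render target.
; Construction creates dynamic snow and footstep materials from depth and strength settings, and BeginPlay creates a white-cleared render target that feeds the snow material.
; SnowHit draws the footstep material onto that target at the hit UV, scaled and rotated to the given rotation, then passes the UV to the snow material.
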(event `self.ReceiveBeginPlay`
  (`self.RenderTarget`))

(event `SnowHit`
  (params (UVLoc :type "Vector2D Structure") (Rotation :type "Float (double-precision)"))
  (bind (_x _y) (`KismetMathLibrary.BreakVector2D` UVLoc))
  (bind (_canvas _size _context) (`KismetRenderingLibrary.BeginDrawCanvasToRenderTarget` (`self.SnowDeformTexture`)))
  (bind (_screen_position _screen_size) (`/Engine/ArtTools/RenderToTexture/Macros/RenderToTextureFunctionLibrary.Set Canvas Material Scale and Position` _size UVLoc (`self.FootstepScale`)))
  (`Canvas.K2_DrawMaterial` _canvas (`self.DynamicFootstep`) _screen_position _screen_size (0.0 0.0) (1.0 1.0) (+ (* Rotation -1.0) -90.0) (0.5 0.5))
  (`MaterialInstanceDynamic.SetVectorParameterValue` (`self.DynamicSnow`) "UV_Transform" (`KismetMathLibrary.MakeColor` _x _y 1.0))
  (`KismetRenderingLibrary.EndDrawCanvasToRenderTarget` _context))

(fn `RenderTarget`
  (bind _returnvalue (`KismetRenderingLibrary.CreateRenderTarget2D` 1024 1024))
  (bind _output_get (set `self.SnowDeformTexture` _returnvalue))
  (`KismetRenderingLibrary.ClearRenderTarget2D` _output_get (struct :`R` 1.0 :`G` 1.0 :`B` 1.0 :`A` 1.0))
  (`MaterialInstanceDynamic.SetTextureParameterValue` (`self.DynamicSnow`) "Dis" _output_get))

(fn `UserConstructionScript`
  (bind _returnvalue (`PrimitiveComponent.CreateDynamicMaterialInstance` (`self.StaticMeshComponent`) 0 "/Game/Deform/M_DeformableMesh.M_DeformableMesh" "None"))
  (bind _output_get (set `self.DynamicSnow` _returnvalue))
  (`MaterialInstanceDynamic.SetScalarParameterValue` _output_get "SnowOffset" (`self.SnowDepth`))
  (bind _returnvalue_2 (`KismetMaterialLibrary.CreateDynamicMaterialInstance` "/Game/Deform/SnowTut/M_Footstep.M_Footstep"))
  (bind _output_get_2 (set `self.DynamicFootstep` _returnvalue_2))
  (`MaterialInstanceDynamic.SetScalarParameterValue` _output_get_2 "Strength" (`self.FootstepStrength`))
  (`MaterialInstanceDynamic.SetScalarParameterValue` _output_get_2 "UpMult" (`self.FootstepUpMulti`)))